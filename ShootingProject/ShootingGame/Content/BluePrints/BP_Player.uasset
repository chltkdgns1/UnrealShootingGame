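; BP_Player is the player Blueprint, moved by input along the world Y (horizontal) and Z (vertical) axes.
; BeginPlay adds the IMC_PlayerInput Enhanced Input mapping context to the first player controller.
; Each axis action offsets the location by its normalized direction, scaled by MoveSpeed and delta time, without sweeping for collision.
; The axes apply independently, so diagonal movement is faster and analog magnitude is discarded.
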(event `self.ReceiveBeginPlay`
  (`EnhancedInputSubsystemInterface.AddMappingContext` (pcsubsystem `EnhancedInputLocalPlayerSubsystem` (`GameplayStatics.GetPlayerController` 0)) "/Game/BluePrints/IMC_PlayerInput.IMC_PlayerInput" 0 (struct)))

(event `EnhancedInput|/Game/BluePrints/IA_Horizontal`
  (params (ActionValue :type "Float (double-precision)") (ElapsedSeconds :type "Float (double-precision)") (TriggeredSeconds :type "Float (double-precision)") (InputAction :type "InputAction Object Reference" :default "/Game/BluePrints/IA_Horizontal.IA_Horizontal"))
  (:`Triggered`
    (`self.K2_SetActorLocation` (+ (* (* (`KismetMathLibrary.Normal` (`KismetMathLibrary.MakeVector` 0.0 ActionValue)) (`self.MoveSpeed`)) (`GameplayStatics.GetWorldDeltaSeconds`)) (`self.K2_GetActorLocation`)))))

(event `EnhancedInput|/Game/BluePrints/IA_Vertical`
  (params (ActionValue :type "Float (double-precision)") (ElapsedSeconds :type "Float (double-precision)") (TriggeredSeconds :type "Float (double-precision)") (InputAction :type "InputAction Object Reference" :default "/Game/BluePrints/IA_Vertical.IA_Vertical"))
  (:`Triggered`
    (`self.K2_SetActorLocation` (+ (* (* (`KismetMathLibrary.Normal` (`KismetMathLibrary.MakeVector` 0.0 0.0 ActionValue)) (`self.MoveSpeed`)) (`GameplayStatics.GetWorldDeltaSeconds`)) (`self.K2_GetActorLocation`)))))

(fn `UserConstructionScript`)